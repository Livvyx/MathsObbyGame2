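; BP_Copter is an actor, filed under FunObstacle, that animates a copter-like object with a moving mesh and a spinning part.
; On BeginPlay, a timeline drives the relative Z location of StaticMesh.
; Each Tick adds a fixed yaw step to StaticMesh02, wrapping at a full turn, so spin speed depends on frame rate.
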(event `self.ReceiveBeginPlay`
  (bind (_direction _z_axis) (`Timeline|Timeline_1` :!via `PlayFromStart`)
    (:`Update`
      (`SceneComponent.K2_SetRelativeLocation` (`self.StaticMesh`) (`KismetMathLibrary.MakeVector` 0.0 0.0 _z_axis) false false))))

(event `self.ReceiveTick`
  (params (DeltaSeconds :type "Float (single-precision)"))
  (`|ExecutionSequence`
    (:`then_0`
      (if (>= (`self.ZRot`) 360.0)
        (set `self.ZRot` 0.0)))
    (:`then_1`
      (bind _output_get (set `self.ZRot` (+ (`self.ZRot`) 40.0)))
      (`SceneComponent.K2_SetRelativeRotation` (`self.StaticMesh02`) (`KismetMathLibrary.MakeRotator` 0.0 0.0 _output_get) false false))))

(fn `UserConstructionScript`)